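; BP_Door is a door actor that can be smashed down once through its DoorCrush event.
; The event checks the player is a BP_FirstPersonCharacter, adds an audio component, disables door collision and uses a dot product to find which side the player is on.
; A Timeline then pitches, slides and drops the door mesh in the direction chosen by that side, and a one-second Delay from its update destroys the actor.
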(event `self.ReceiveTick`
  (params (DeltaSeconds :type "Float (single-precision)")))

(event `/Game/My/doorCrush.DoorCrush`
  (params (CharVectorIn :type "Vector Structure") (CharLocIn :type "Vector Structure"))
  (bind _11door (`self.11door`))
  (bind _11door_2 (`self.11door`))
  (`/Engine/EditorBlueprintResources/StandardMacros.IsValid` (`self.11door`)
    (:`Is Valid`
      (bind _asbp_first_person_character (cast `/Game/FirstPerson/Blueprints/BP_FirstPersonCharacter` (`GameplayStatics.GetPlayerPawn` 0)))
      (if (`self.Condition`)
        (set `self.Condition` false)
        (`AddComponent|NODE_AddAudioComponent-2`)
        (`PrimitiveComponent.SetCollisionEnabled` (`self.11door`) "NoCollision")
        (set `self.Condition_0` (> (`KismetMathLibrary.Dot_VectorVector` (`SceneComponent.GetForwardVector` (`self.11door`)) (`KismetMathLibrary.GetDirectionUnitVector` (`self.K2_GetActorLocation`) (`self.K2_GetActorLocation` _asbp_first_person_character))) 0.0))
        (bind (_direction _newtrack_0 _newtrack_1) (`Timeline|Timeline`)
          (:`Update`
            (if (`self.Condition_0`)
              (`SceneComponent.K2_SetRelativeRotation` _11door_2 (`KismetMathLibrary.MakeRotator` 0.0 (`KismetMathLibrary.Lerp` 0.0 90.0 _newtrack_0)) false false)
              (bind _returnvalue (`KismetMathLibrary.Lerp` 0.0 -100.0 _newtrack_1))
              (`SceneComponent.K2_SetRelativeLocation` _11door_2 (`KismetMathLibrary.MakeVector` (`KismetMathLibrary.Lerp` 0.0 -500.0 _newtrack_0) 0.0 _returnvalue) false false)
              (`KismetSystemLibrary.Delay` 1.0)
              (`self.K2_DestroyActor`)
              (else
                (`SceneComponent.K2_SetRelativeRotation` _11door (`KismetMathLibrary.MakeRotator` 0.0 (`KismetMathLibrary.Lerp` 0.0 -90.0 _newtrack_0)) false false)
                (`SceneComponent.K2_SetRelativeLocation` _11door (`KismetMathLibrary.MakeVector` (`KismetMathLibrary.Lerp` 0.0 500.0 _newtrack_0) 0.0 _returnvalue) false false)
                (`KismetSystemLibrary.Delay` 1.0)
                (`self.K2_DestroyActor`)))))))))

(fn `UserConstructionScript`)