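; BP_dog is an AI-driven dog that chases the player.
; It stores the player character on BeginPlay and issues AI Move To toward it every Tick.
; When its Sphere overlaps BP_FirstPersonCharacter, it sends PomerChelMessage to all actors implementing the DoorOpen interface.
; An upward line trace and the pass-through NewDodInter function are unconnected leftovers.
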(event `self.ReceiveBeginPlay`
  (bind _output_get (set `self.NewVar` (`GameplayStatics.GetPlayerCharacter` 0))))

(event `self.ReceiveTick`
  (params (DeltaSeconds :type "Float (single-precision)"))
  (`|AIMoveTo` null (0.0 0.0 0.0) (stale `self.ReceiveBeginPlay` _output_get)))

(event `self.Sphere.OnComponentBeginOverlap`
  (params (OverlappedComponent :type "PrimitiveComponent Object Reference") (OtherActor :type "Actor Object Reference") (OtherComp :type "PrimitiveComponent Object Reference") (OtherBodyIndex :type Integer) (bFromSweep :type Boolean) (SweepResult :type "HitResult Structure (by ref)"))
  (cast `/Game/FirstPerson/Blueprints/BP_FirstPersonCharacter` OtherActor)
  (bind _outactors (`GameplayStatics.GetAllActorsWithInterface` "/Game/My/DoorOpen.DoorOpen_C"))
  (message `/Game/My/DoorOpen.pomerChel` _outactors))

(fn `NewDodInter`
  (params (NewParam :type "Actor Object Reference"))
  (returns (NewParam1 :type "Actor Object Reference"))
  (return NewParam))

(fn `UserConstructionScript`)