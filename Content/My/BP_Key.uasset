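; BP_Key is a key pickup actor that reacts once to overlap, then removes itself without passing anything to the player.
; A boolean gate clears before the cast to BP_FirstPersonCharacter, so any first overlapping actor uses it up.
; For the player, it adds an audio component, animates the key's scale with a timeline and destroys the actor after a short delay.
; An unconnected timeline for vertical bobbing never runs.
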(event `self.ReceiveBeginPlay`)

(event `self.ReceiveActorBeginOverlap`
  (params (OtherActor :type "Actor Object Reference"))
  (if (`self.NewVar`)
    (set `self.NewVar` false)
    (cast `/Game/FirstPerson/Blueprints/BP_FirstPersonCharacter` OtherActor)
    (`AddComponent|NODE_AddAudioComponent-0`)
    (bind (_direction _newtrack_0) (`Timeline|Timeline_0`)
      (:`Update`
        (`SceneComponent.SetRelativeScale3D` (`self.key`) (`KismetMathLibrary.Conv_DoubleToVector` _newtrack_0))
        (`KismetSystemLibrary.Delay` 2.0)
        (`self.K2_DestroyActor`)))))

(fn `UserConstructionScript`)